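; Player character Blueprint handling fire feedback, third-person body rotation and a full-minimap toggle on M.
; Left mouse runs a recoil timeline with randomly mirrored yaw and loops camera shake until release or CheckFire fails on empty ammo or reload.
; Tick turns the mesh toward movement input and the actor toward camera yaw, or straightens the mesh while zoomed.
; Tick also prints camera yaw for debugging.
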(event `self.ReceiveTick`
  (params (DeltaSeconds :type "Float (single-precision)"))
  (bind (_returnvalue_roll _returnvalue_pitch _returnvalue_yaw) (`KismetMathLibrary.BreakRotator` (`KismetMathLibrary.Quat_Rotator` (`KismetMathLibrary.Conv_VectorToQuaternion` (`SceneComponent.GetForwardVector` (`self.ThirdPersonCameraComponent`))))))
  ;[1 1 1] 3인칭 회전 보정 값
  (`self.ThirdPersonMotionCompensate` DeltaSeconds)
  (`KismetSystemLibrary.PrintString` (`KismetStringLibrary.Conv_DoubleToString` _returnvalue_yaw)))

(event `Key|LeftMouseButton`
  (params (Key :type "Key Structure"))
  (bind _returnvalue (`GameplayStatics.GetPlayerController` 0))
  ;[1 1 1] 총 반동 및 카메라 흔들림
  (:`Pressed`
    (`|ExecutionSequence`
      (:`then_0`
        (set `self.IsRand` (`KismetMathLibrary.RandomBool`))
        (bind _ischeck (`self.Check Fire`))
        (if _ischeck
          (set `self.IsFire` true)
          (`|ExecutionSequence`
            (:`then_0`
              (bind (_direction _pitch _yaw) (`Timeline|Recoil` :!via `PlayFromStart` :!label _label)
                (:`Update`
                  (`PlayerController.AddPitchInput` _returnvalue _pitch)
                  (if (`self.IsRand`)
                    (`PlayerController.AddYawInput` _returnvalue _yaw)
                    (else
                      (`PlayerController.AddYawInput` _returnvalue (* _yaw -1.0)))))))
            (:`then_1`
              (`GameplayStatics.PlayWorldCameraShake` "/Game/Blueprint/Game/CameraShake/BP_FireCameraShake.BP_FireCameraShake_C" (`self.K2_GetActorLocation`) 0.0 150.0 :!label _label_2)
              (`KismetSystemLibrary.Delay` 0.1)
              (bind _ischeck_2 (`self.Check Fire`))
              (if _ischeck_2
                (if (`self.IsFire`)
                  (goto _label_2)))))
          (else
            (set `self.IsFire` false :!label _label_3)
            (goto _label :!via `Stop`))))))
  (:`Released`
    (goto _label_3)))

(event `Empty Ammo`
  ;[1 1 1] 총 반동 및 카메라 흔들림
  (goto _label :!via `Stop`))

(event `Key|M`
  (params (Key :type "Key Structure"))
  ;[1 1 1] 미니맵
  (:`Pressed`
    (`/Engine/EditorBlueprintResources/StandardMacros.FlipFlop`
      (:`A`
        (bind _returnvalue (`|CreateWidget` "/Game/Blueprint/Widget/W_MinimapEntire.W_MinimapEntire_C"))
        (`UserWidget.AddToViewport` _returnvalue 0))
      (:`B`
        (`Widget.RemoveFromParent` _returnvalue)))))

(fn `Check Fire`
  (returns (IsCheck :type Boolean))
  (bind _returnvalue (`self.GetCurrentAmmo`))
  (if (<= _returnvalue 0)
    (`self.Empty Ammo`)
    (else
      (bind _returnvalue_2 (`self.GetIsReload`))
      (if _returnvalue_2
        (`self.Empty Ammo`)
        (else
          (return true)))))
  (return false))

(fn `ThirdPersonMotionCompensate`
  (params (DeltaTime :type "Float (double-precision)"))
  (bind _returnvalue (`self.GetInputAxisValue`))
  (bind _returnvalue_2 (`self.GetInputAxisValue`))
  (bind _tps_mesh (`self.TPS_Mesh`))
  (bind _returnvalue_3 (`SceneComponent.GetRelativeTransform` _tps_mesh))
  (bind (_returnvalue_roll _returnvalue_pitch _returnvalue_yaw) (`KismetMathLibrary.BreakRotator` (`KismetMathLibrary.Quat_Rotator` (`KismetMathLibrary.Conv_VectorToQuaternion` (`SceneComponent.GetForwardVector` (`self.ThirdPersonCameraComponent`))))))
  (bind (_returnvalue_roll_2 _returnvalue_pitch_2 _returnvalue_yaw_2) (`KismetMathLibrary.BreakRotator` (`KismetMathLibrary.Quat_Rotator` (`KismetMathLibrary.Conv_VectorToQuaternion` (`KismetMathLibrary.Conv_Vector2DToVector` (`KismetMathLibrary.MakeVector2D` _returnvalue _returnvalue_2) 1.0)))))
  (bind _returnvalue_4 (`self.GetIsZoomin`))
  (if (not _returnvalue_4)
    (if (not (and (== _returnvalue 0.0) (== _returnvalue_2 0.0)))
      (`SceneComponent.K2_SetRelativeRotation` _tps_mesh (`KismetMathLibrary.MakeRotator` 0.0 0.0 (.yaw (.rotation (`KismetMathLibrary.TInterpTo` _returnvalue_3 (`KismetMathLibrary.MakeTransform` (0.0 0.0 0.0) (`KismetMathLibrary.MakeRotator` 0.0 0.0 (+ _returnvalue_yaw_2 -90.0))) DeltaTime 11.25)))) false false)
      (`self.K2_SetActorRotation` (`KismetMathLibrary.MakeRotator` 0.0 0.0 _returnvalue_yaw)))
    (else
      (`SceneComponent.K2_SetRelativeRotation` _tps_mesh (`KismetMathLibrary.MakeRotator` 0.0 0.0 (.yaw (.rotation (`KismetMathLibrary.TInterpTo` _returnvalue_3 (`KismetMathLibrary.MakeTransform` (0.0 0.0 0.0) (`KismetMathLibrary.MakeRotator` 0.0 0.0 -90.0)) DeltaTime 22.5)))) false false))))

(fn `UserConstructionScript`)